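; BP_Enemy is an AI enemy that chases the player and, on capsule overlap, drags them to a drop-off point.
; Tick re-issues AIMoveTo toward either the player or, while dragging with input disabled, the character's DragLocation.
; On arrival it detaches the player, flags AtDropOff, teleports to its spawn point, restores input and starts a drag cooldown.
; The enemy only sets BeingDragged and never attaches the player itself.
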(event OnComponentBeginOverlap(CapsuleComponent)
  (params (OverlappedComponent :type Primitive%20Component%20Object%20Reference) (OtherActor :type Actor%20Object%20Reference) (OtherComp :type Primitive%20Component%20Object%20Reference) (OtherBodyIndex :type Integer) (bFromSweep :type Boolean) (SweepResult :type Hit%20Result%20Structure%20%28by%20ref%29))
  ;[1 1 1] On Overlap With Player, Sets Dragging to True
  (bind _asfirst_person_character (Utilities|Casting|CastToFirstPersonCharacter OtherActor))
  (if (Variables|Default|GetcanDrag)
    (if (not (Variables|Default|GetisDragging))
      (Variables|Default|SetisDragging true)
      (Variables|/Game/FirstPersonCPP/Blueprints/FirstPersonCharacter.FirstPersonCharacter_C|SetbeingDragged _asfirst_person_character true))))

(event OnComponentEndOverlap(CapsuleComponent)
  (params (OverlappedComponent :type Primitive%20Component%20Object%20Reference) (OtherActor :type Actor%20Object%20Reference) (OtherComp :type Primitive%20Component%20Object%20Reference) (OtherBodyIndex :type Integer))
  ;[1 1 1] On End Overlap With Player, Sets Dragging To False
  (if (not (Variables|Default|GetisDragging))
    (bind _asfirst_person_character (Utilities|Casting|CastToFirstPersonCharacter OtherActor))
    (Variables|/Game/FirstPersonCPP/Blueprints/FirstPersonCharacter.FirstPersonCharacter_C|SetbeingDragged _asfirst_person_character false)))

(event EventBeginPlay
  ;[1 1 1] Sets Return Location To Spawn Position
  (Variables|Default|SetreturnLoc (Transformation|GetActorLocation)))

(event EventTick
  (params (DeltaSeconds :type Float%20%28single-precision%29))
  (bind _returnvalue (Game|Player|GetPlayerPawn 0))
  ;[1 1 1] Checks If The Enemy Is Dragging, Or Has Finished Dragging, The Player
  (if (Variables|Default|GetisDragging)
    ;[1 1 1] Disables Player Input And Moves to Drop-off Location
    (Input|DisableInput _returnvalue 0)
    (bind _asfirst_person_character (Utilities|Casting|CastToFirstPersonCharacter _returnvalue))
    (AI|AIMoveTo self (Variables|/Game/FirstPersonCPP/Blueprints/FirstPersonCharacter.FirstPersonCharacter_C|GetDrag%20Location _asfirst_person_character) 0 5.0 false
      (:OnSuccess
        (Collision|SetActorEnableCollision _asfirst_person_character true)
        (Transformation|DetachFromActor _asfirst_person_character "KeepWorld" "KeepWorld" "KeepWorld")
        (Variables|Default|SetisDragging false)
        (Variables|/Game/FirstPersonCPP/Blueprints/FirstPersonCharacter.FirstPersonCharacter_C|SetatDropOff _asfirst_person_character true)
        (Variables|Default|SetgoToStart true)
        (Utilities|FlowControl|Delay (Variables|Default|GetDragCooldown))
        (Variables|Default|SetcanDrag true)))
    (elif (Variables|Default|GetgoToStart)
      ;[1 1 1] Teleports Back To The Start
      (Transformation|SetActorLocation self (Variables|Default|GetreturnLoc) false false)
      (Input|EnableInput (Game|Player|GetPlayerPawn 0) 0)
      (Variables|Default|SetgoToStart false)
      (else
        ;[1 1 1] Constantly Moves To Player
        (AI|AIMoveTo self "0, 0, 0" (Game|Player|GetPlayerPawn 0) 5.0 false)))))

(fn ConstructionScript)