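; BP_Fridge is a fridge that swings its door open when the player has entered the matching number code, also marking the fridge quest complete.
; Every tick it compares its code with the number stored on the first-person character, then sets the open flag and plays a timeline that rotates the door's yaw by a set angle.
; A trigger box tracks whether something is in range, but the code check does not use it.
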(event OnComponentBeginOverlap(TriggerBox)
  (params (OverlappedComponent :type Primitive%20Component%20Object%20Reference) (OtherActor :type Actor%20Object%20Reference) (OtherComp :type Primitive%20Component%20Object%20Reference) (OtherBodyIndex :type Integer) (bFromSweep :type Boolean) (SweepResult :type Hit%20Result%20Structure%20%28by%20ref%29))
  (Variables|Default|SetisInRange true))

(event OnComponentEndOverlap(TriggerBox)
  (params (OverlappedComponent :type Primitive%20Component%20Object%20Reference) (OtherActor :type Actor%20Object%20Reference) (OtherComp :type Primitive%20Component%20Object%20Reference) (OtherBodyIndex :type Integer))
  (Variables|Default|SetisInRange false))

(event EventTick
  (params (DeltaSeconds :type Float%20%28single-precision%29))
  ;[1 1 1] Checks if the Player code input is correct
  (bind _asfirst_person_character (Utilities|Casting|CastToFirstPersonCharacter (Game|Player|GetPlayerPawn 0)))
  (if (== (Variables|Default|GetnumCode) (Variables|/Game/FirstPersonCPP/Blueprints/FirstPersonCharacter.FirstPersonCharacter_C|GetnumberEntered _asfirst_person_character))
    (Variables|Default|SetisFridgeOpen true)
    (Variables|/Game/FirstPersonCPP/Blueprints/FirstPersonCharacter.FirstPersonCharacter_C|SetFridgeQuestComp _asfirst_person_character true)
    (bind _newtrack_0 (Timeline|Timeline_0 Play)
      (:Update
        (Transformation|SetRelativeRotation (Variables|Default|Getfridge_door) (Math|Rotator|MakeRotator 0.0 0.0 (* _newtrack_0 (Variables|Default|Getangle))) false false)))))

(fn ConstructionScript)