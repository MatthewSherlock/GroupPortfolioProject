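; Main menu light actor that flickers a spot light and a point light at irregular intervals.
; On BeginPlay it caches the spot light's intensity as the base, then plays a timeline that scales both lights by its intensity curve.
; When the timeline finishes, it waits a random few seconds and restarts the flicker, looping indefinitely.
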(event Custom|StartFlickering
  (bind _intensity (Timeline|FlickeringTimeline PlayFromStart)
    (:Update
      (Rendering|Components|Light|SetIntensity (Variables|Default|GetSpotLight) (* _intensity (Variables|Default|GetlightIntensity)))
      (Rendering|Components|Light|SetIntensity (Variables|Default|GetPointLight) (* _intensity (Variables|Default|GetlightIntensity))))
    (:Finished
      (Utilities|FlowControl|Delay (Math|Random|RandomFloatinRange 2.0 1e+01))
      (CallFunction|StartFlickering))))

(event EventBeginPlay
  (Variables|Default|SetlightIntensity (Variables|/Script/Engine.LightComponentBase|GetIntensity (Variables|Default|GetSpotLight)))
  (CallFunction|StartFlickering))

(fn ConstructionScript)