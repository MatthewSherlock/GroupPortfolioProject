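; BP_EndDoor is an end-of-game door actor that shows the WinUI widget once it becomes active.
; Tick polls DoorActive, which is not set in this Blueprint, and uses a DoOnce to create the widget a single time.
; TriggerBox overlaps with FirstPersonCharacter set PlayerAtDoor to true on both begin and end, and Tick does not check that flag.
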(event OnComponentEndOverlap(TriggerBox)
  (params (OverlappedComponent :type Primitive%20Component%20Object%20Reference) (OtherActor :type Actor%20Object%20Reference) (OtherComp :type Primitive%20Component%20Object%20Reference) (OtherBodyIndex :type Integer))
  (Utilities|Casting|CastToFirstPersonCharacter OtherActor)
  (Variables|Default|SetplayerAtDoor true))

(event OnComponentBeginOverlap(TriggerBox)
  (params (OverlappedComponent :type Primitive%20Component%20Object%20Reference) (OtherActor :type Actor%20Object%20Reference) (OtherComp :type Primitive%20Component%20Object%20Reference) (OtherBodyIndex :type Integer) (bFromSweep :type Boolean) (SweepResult :type Hit%20Result%20Structure%20%28by%20ref%29))
  (Utilities|Casting|CastToFirstPersonCharacter OtherActor)
  (Variables|Default|SetplayerAtDoor true))

(event EventBeginPlay)

(event Collision|EventActorBeginOverlap
  (params (OtherActor :type Actor%20Object%20Reference)))

(event EventTick
  (params (DeltaSeconds :type Float%20%28single-precision%29))
  (if (Variables|Default|GetDoorActive)
    (Utilities|FlowControl|DoOnce false
      (:Completed
        (bind _returnvalue (UserInterface|CreateWidget "/Game/UI/WinUI.WinUI_C"))
        (UserInterface|Viewport|AddtoViewport _returnvalue 0)))))

(fn ConstructionScript)