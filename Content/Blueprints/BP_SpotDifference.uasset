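; BP_SpotDifference is a spot-the-difference puzzle actor that reveals a hidden Code component once the odd one out is found.
; BeginPlay hides the code and clears the found flag.
; A TriggerBox overlap prints a debug message for any actor, but sets the flag only for the FirstPersonCharacter.
; Tick polls that flag and, while it is set, makes the code visible every frame.
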(event OnComponentBeginOverlap(TriggerBox)
  (params (OverlappedComponent :type Primitive%20Component%20Object%20Reference) (OtherActor :type Actor%20Object%20Reference) (OtherComp :type Primitive%20Component%20Object%20Reference) (OtherBodyIndex :type Integer) (bFromSweep :type Boolean) (SweepResult :type Hit%20Result%20Structure%20%28by%20ref%29))
  (Development|PrintString "Spot the Difference Trigger Active")
  (Utilities|Casting|CastToFirstPersonCharacter OtherActor)
  (Variables|Default|SetoddOneOutFound true))

(event EventBeginPlay
  (Rendering|SetVisibility (Variables|Default|GetCode) false false)
  (Variables|Default|SetoddOneOutFound false))

(event Collision|EventActorBeginOverlap
  (params (OtherActor :type Actor%20Object%20Reference)))

(event EventTick
  (params (DeltaSeconds :type Float%20%28single-precision%29))
  (if (Variables|Default|GetoddOneOutFound)
    (Rendering|SetVisibility (Variables|Default|GetCode) true false)))

(fn ConstructionScript)